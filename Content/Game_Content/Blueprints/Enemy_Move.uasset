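; Side-scrolling patrol enemy that walks along the X axis and hurts the Octopus on contact.
; Tick feeds movement input in the current direction and yaws the sprite to match.
; Any capsule hit reverses direction, as the Octopus cast runs after the flip and gates nothing.
; Sphere overlap calls the Octopus's DamageSystem, while the Damage event lowers enemy health and destroys the actor at zero or below.
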(event OnComponentHit(CapsuleComponent)
  (params (HitComponent :type Primitive%20Component%20Object%20Reference) (OtherActor :type Actor%20Object%20Reference) (OtherComp :type Primitive%20Component%20Object%20Reference) (NormalImpulse :type Vector :default "0, 0, 0") (Hit :type Hit%20Result%20Structure%20%28by%20ref%29))
  ;[1 1 1] Rotates Enemy If Hit player
  (Variables|Default|SetbisMovingRight (not (Variables|Default|GetbisMovingRight)))
  (Utilities|Casting|CastToOctopus OtherActor))

(event OnComponentBeginOverlap(Sphere)
  (params (OverlappedComponent :type Primitive%20Component%20Object%20Reference) (OtherActor :type Actor%20Object%20Reference) (OtherComp :type Primitive%20Component%20Object%20Reference) (OtherBodyIndex :type Integer) (bFromSweep :type Boolean) (SweepResult :type Hit%20Result%20Structure%20%28by%20ref%29))
  (bind _asoctopus (Utilities|Casting|CastToOctopus OtherActor))
  (Default|DamageSystem _asoctopus 0.1))

(event Custom|Damage
  (params (Damage%20Given :type Integer))
  (bind _output_get (Variables|Default|SetEnemy%20Health (- (Variables|Default|GetEnemy%20Health) Damage%20Given)))
  (if (<= _output_get 0)
    (Actor|DestroyActor)))

(event Custom|Direction
  ;[1 1 1] Makes AI move
  (Transformation|SetRelativeRotation (Variables|Default|GetSprite) (Math|Rotator|MakeRotator 0.0 0.0 (Math|Float|SelectFloat 0.0 1.8e+02 (Variables|Default|GetbisMovingRight))) false false)
  (Pawn|Input|AddMovementInput (Math|Vector|SelectVector "1.000000, 0, 0" "-1.000000, 0, 0" (Variables|Default|GetbisMovingRight)) 1.0 false))

(event EventTick
  (params (DeltaSeconds :type Float%20%28single-precision%29))
  (CallFunction|Direction))

(fn ConstructionScript)